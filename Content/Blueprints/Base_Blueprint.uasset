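; Base_Blueprint is a damageable actor that loses health when hit by AI bullets and is destroyed when health runs out.
; Its Box overlap checks for the BulletAI tag, applies fixed damage to itself and destroys the bullet.
; The AnyDamage event subtracts truncated damage from HealthPoints and destroys the actor at zero or below.
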(event `self.ReceiveAnyDamage`
  (params (Damage :type "Float (single-precision)") (DamageType :type "DamageType Object Reference") (InstigatedBy :type "Controller Object Reference") (DamageCauser :type "Actor Object Reference"))
  (bind _output_get (set `self.HealthPoints` (- (`self.HealthPoints`) (`KismetMathLibrary.FTrunc` Damage))))
  (if (<= _output_get 0)
    (`self.K2_DestroyActor`)))

(event `self.Box.OnComponentBeginOverlap`
  (params (OverlappedComponent :type "PrimitiveComponent Object Reference") (OtherActor :type "Actor Object Reference") (OtherComp :type "PrimitiveComponent Object Reference") (OtherBodyIndex :type Integer) (bFromSweep :type Boolean) (SweepResult :type "HitResult Structure (by ref)"))
  (if (`self.ActorHasTag` OtherActor "BulletAI")
    (`GameplayStatics.ApplyDamage` self 10.0 null OtherActor)
    (`self.K2_DestroyActor` OtherActor)))

(fn `UserConstructionScript`)